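; Mutant enemy character that chases Our_Hero, hurts it at close range and dies from any damage taken.
; PawnSensing sightings trigger an AI MoveTo toward the hero.
; Sphere overlap starts a looping timer that calls the hero's Damage function, and actor end-overlap pauses it.
; Taking damage plays the dying animation, detaches the controller and destroys the actor after a delay.
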(event `self.ReceiveActorEndOverlap`
  (params (OtherActor :type "Actor Object Reference"))
  ;[1 1 1] Hurt the Hero
  (cast `/Game/BluePrints/Our_Hero` OtherActor)
  (`KismetSystemLibrary.K2_PauseTimer` null "Monster Damage"))

(event `self.Sphere.OnComponentBeginOverlap`
  (params (OverlappedComponent :type "PrimitiveComponent Object Reference") (OtherActor :type "Actor Object Reference") (OtherComp :type "PrimitiveComponent Object Reference") (OtherBodyIndex :type Integer) (bFromSweep :type Boolean) (SweepResult :type "HitResult Structure (by ref)"))
  ;[1 1 1] Hurt the Hero
  (cast `/Game/BluePrints/Our_Hero` OtherActor)
  (`KismetSystemLibrary.K2_SetTimer` null "Monster Damage" 3.0 true 0.3))

(event `self.PawnSensing.OnSeePawn`
  (params (Pawn :type "Pawn Object Reference"))
  ;[1 1 1] AI Find Player
  (bind _asour_hero (cast `/Game/BluePrints/Our_Hero` Pawn))
  (`|AIMoveTo` self (0.0 0.0 0.0) _asour_hero))

(event `self.ReceiveAnyDamage`
  (params (Damage :type "Float (single-precision)") (DamageType :type "DamageType Object Reference") (InstigatedBy :type "Controller Object Reference") (DamageCauser :type "Actor Object Reference"))
  ;[1 1 1] Death and Remove from level
  (`SkeletalMeshComponent.PlayAnimation` (`self.Mesh`) "/Game/CharacterAssets/Enemies/Muts/Anim/mutant_dying.mutant_dying" false)
  (`self.DetachFromControllerPendingDestroy`)
  (`KismetSystemLibrary.Delay` 10.0)
  (`self.K2_DestroyActor`))

(fn `Monster Damage`
  (bind _asour_hero (cast `/Game/BluePrints/Our_Hero` (`GameplayStatics.GetPlayerCharacter` 0)))
  (`/Game/BluePrints/Our_Hero.Damage` _asour_hero))

(fn `UserConstructionScript`)