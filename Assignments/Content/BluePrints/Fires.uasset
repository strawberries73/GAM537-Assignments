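; Fires is a Blueprint that drives a PointLight's intensity, apparently as a fire light flicker.
; BeginPlay sets the light to MaxIntensity.
; Tick uses a FlipFlop to alternate between MaxIntensity and MinIntenstity, gated on DeltaSeconds modulo 10 equalling zero.
; That gate tests frame delta rather than elapsed time, so it rarely, if ever, passes in normal play.
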(event `self.ReceiveBeginPlay`
  (`LightComponent.SetIntensity` (`self.PointLight`) (`KismetMathLibrary.Conv_IntToDouble` (`self.max_Intensity`))))

(event `self.ReceiveTick`
  (params (DeltaSeconds :type "Float (single-precision)"))
  (if (== (mod DeltaSeconds 10.0) 0.0)
    (`/Engine/EditorBlueprintResources/StandardMacros.FlipFlop`
      (:`A`
        (`LightComponent.SetIntensity` (`self.PointLight`) (`KismetMathLibrary.Conv_IntToDouble` (`self.max_Intensity`))))
      (:`B`
        (`LightComponent.SetIntensity` (`self.PointLight`) (`KismetMathLibrary.Conv_IntToDouble` (`self.min_Intenstity`)))))))

(fn `UserConstructionScript`)