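; Master Mutant is an enemy pawn that spins in place while looking, then chases the hero on sight and plays a swipe attack on arrival.
; Damage to the hero comes from a looping timer, started on sphere overlap and paused when actor overlap ends.
; Hits trigger a pain stagger until a hit threshold causes death, controller detachment, delayed destruction and a final HUD message.
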(event `self.ReceiveActorEndOverlap`
  (params (OtherActor :type "Actor Object Reference"))
  ;[1 1 1] Damage the Hero
  (cast `/Game/BluePrints/Our_Hero` OtherActor)
  (`KismetSystemLibrary.K2_PauseTimer` null "Monster Damage"))

(event `self.Sphere.OnComponentBeginOverlap`
  (params (OverlappedComponent :type "PrimitiveComponent Object Reference") (OtherActor :type "Actor Object Reference") (OtherComp :type "PrimitiveComponent Object Reference") (OtherBodyIndex :type Integer) (bFromSweep :type Boolean) (SweepResult :type "HitResult Structure (by ref)"))
  ;[1 1 1] Damage the Hero
  (cast `/Game/BluePrints/Our_Hero` OtherActor)
  (`KismetSystemLibrary.K2_SetTimer` null "Monster Damage" 3.0 true 0.3))

(event `self.PawnSensing.OnSeePawn`
  (params (Pawn :type "Pawn Object Reference"))
  ;[1 1 1] AI
  (set `self.Looking` false)
  (if (`self.Can Move`)
    (bind _asour_hero (cast `/Game/BluePrints/Our_Hero` Pawn))
    (`|AIMoveTo` self (0.0 0.0 0.0) _asour_hero 100.0 true
      (:`OnSuccess`
        ;[1 1 1] Attack
        (set `self.Can Move` false)
        (`self.PlayAnimMontage` "/Game/CharacterAssets/Enemies/Leader/Anim/mutant_swiping_Montage.mutant_swiping_Montage")
        (`KismetSystemLibrary.Delay` 2.0)
        (set `self.Can Move` true)
        (set `self.Looking` true)))))

(event `self.ReceiveAnyDamage`
  (params (Damage :type "Float (single-precision)") (DamageType :type "DamageType Object Reference") (InstigatedBy :type "Controller Object Reference") (DamageCauser :type "Actor Object Reference"))
  (if (>= (`self.Hit Count`) (`self.Hits needed`))
    ;[1 1 1] Death
    (`SkeletalMeshComponent.PlayAnimation` (`self.Mesh`) "/Game/CharacterAssets/Enemies/Leader/Anim/Standing_Death_Left_01.Standing_Death_Left_01" false)
    (`self.DetachFromControllerPendingDestroy`)
    (`KismetSystemLibrary.Delay` 10.0)
    (`self.K2_DestroyActor`)
    (bind _returnvalue (`|CreateWidget` "/Game/BluePrints/Our_Text_Hud.Our_Text_Hud_C" (`GameplayStatics.GetPlayerController` 0)))
    (bind _output_get (set `self.Dialogue` _returnvalue))
    (`UserWidget.AddToViewport` _output_get 0)
    (set `/Game/BluePrints/Our_Text_Hud.Dialogue Text` (`self.Final Message`) _output_get)
    (else
      ;[1 1 1] Pain
      (set `self.Can Move` false)
      (`self.PlayAnimMontage` "/Game/CharacterAssets/Enemies/Leader/Anim/Pain_Gesture_Montage.Pain_Gesture_Montage")
      (set `self.Hit Count` (+ (`self.Hit Count`) 1))
      (`KismetSystemLibrary.Delay` 2.0)
      (set `self.Can Move` true))))

(event `self.ReceiveTick`
  (params (DeltaSeconds :type "Float (single-precision)"))
  (if (`self.Looking`)
    (`self.K2_AddActorWorldRotation` (struct :`Yaw` 2.0))))

(fn `Monster Damage`
  (bind _asour_hero (cast `/Game/BluePrints/Our_Hero` (`GameplayStatics.GetPlayerCharacter` 0)))
  (`/Game/BluePrints/Our_Hero.Damage` _asour_hero))

(fn `UserConstructionScript`)