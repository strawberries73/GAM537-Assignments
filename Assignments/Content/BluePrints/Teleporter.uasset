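; Teleporter is an interactable that opens the next level once the player has collected enough relics.
; On Interact it compares RelicsCount from the Hero_GI game instance against RelicsNeeded and, if met, loads NextLevel by name.
; Otherwise it toggles an Our_Text_Hud dialogue widget showing MyText, removing it if already displayed.
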(event `/Game/BluePrints/Interact_I.Interact`
  (bind _ashero_gi (cast `/Game/BluePrints/Hero_GI` (`GameplayStatics.GetGameInstance`)))
  (if (>= (`/Game/BluePrints/Hero_GI.Relics Count` _ashero_gi) (`self.Relics Needed`))
    ;[1 1 1] Go to next level
    (`GameplayStatics.OpenLevel` (`self.Next Level`))
    (else
      ;[1 1 1] Display Text
      (`/Engine/EditorBlueprintResources/StandardMacros.IsValid` (`self.Dialogue`)
        (:`Is Valid`
          (`Widget.RemoveFromParent` (`self.Dialogue`))
          (set `self.Dialogue` null))
        (:`Is Not Valid`
          (bind _returnvalue (`|CreateWidget` "/Game/BluePrints/Our_Text_Hud.Our_Text_Hud_C" (`GameplayStatics.GetPlayerController` 0)))
          (bind _output_get (set `self.Dialogue` _returnvalue))
          (`UserWidget.AddToViewport` _output_get 0)
          (set `/Game/BluePrints/Our_Text_Hud.Dialogue Text` (`self.My_text`) (`self.Dialogue`)))))))

(fn `UserConstructionScript`)