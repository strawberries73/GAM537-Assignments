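; Relic_BP is a collectible relic pickup that spins in the world until the hero touches it.
; On BeginPlay it caches the Hero_GI game instance.
; An overlap by Our_Hero increments RelicsCount on that game instance, then destroys the relic.
; Tick adds a fixed world rotation every frame without delta-time scaling, so spin speed depends on frame rate.
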(event `self.ReceiveBeginPlay`
  (bind _ashero_gi (cast `/Game/BluePrints/Hero_GI` (`GameplayStatics.GetGameInstance`)))
  (set `self.Hero_GI` _ashero_gi))

(event `self.ReceiveActorBeginOverlap`
  (params (OtherActor :type "Actor Object Reference"))
  (bind _hero_gi (`self.Hero_GI`))
  (cast `/Game/BluePrints/Our_Hero` OtherActor)
  (set `/Game/BluePrints/Hero_GI.Relics Count` (+ (`/Game/BluePrints/Hero_GI.Relics Count` _hero_gi) 1) _hero_gi)
  (`self.K2_DestroyActor`))

(event `self.ReceiveTick`
  (params (DeltaSeconds :type "Float (single-precision)"))
  (`self.K2_AddActorWorldRotation` (struct :`Yaw` 2.0)))

(fn `UserConstructionScript`)