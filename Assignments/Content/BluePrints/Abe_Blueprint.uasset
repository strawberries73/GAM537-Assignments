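; Abe is an interactable that toggles an on-screen dialogue, apparently as a talking NPC.
; Interact creates an Our_Text_Hud widget for the first player, adds it to the viewport and fills its DialogueText from the Speech variable.
; Interacting again while the widget is valid removes and clears it, with IsTalking tracking the open or closed state.
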(event `/Game/BluePrints/Interact_I.Interact`
  (`/Engine/EditorBlueprintResources/StandardMacros.IsValid` (`self.Dialogue`)
    (:`Is Valid`
      (set `self.is talking?` false)
      (`Widget.RemoveFromParent` (`self.Dialogue`))
      (set `self.Dialogue` null))
    (:`Is Not Valid`
      (set `self.is talking?` true)
      (bind _returnvalue (`|CreateWidget` "/Game/BluePrints/Our_Text_Hud.Our_Text_Hud_C" (`GameplayStatics.GetPlayerController` 0)))
      (bind _output_get (set `self.Dialogue` _returnvalue))
      (`UserWidget.AddToViewport` _output_get 0)
      (set `/Game/BluePrints/Our_Text_Hud.Dialogue Text` (`self.Speech`) (`self.Dialogue`)))))

(fn `UserConstructionScript`)